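; BP_PatrolAI is an AI character that endlessly patrols actors tagged PatrolPoint in random order.
; BeginPlay gathers and shuffles the points and randomizes walk speed.
; GoToPatrolPoints chains AIMoveTo calls, advancing on success or failure and reshuffling after each full round, with a delay only between points within a round.
; A self-repeating MoveTo event that chases the player is defined but not called here.
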(event Custom|MoveTo
  (AI|AIMoveTo self "0, 0, 0" (Game|GetPlayerCharacter 0) 2e+02 false ; Moves to player location
    (:OnSuccess
      (Development|PrintString "Found Player"))
    (:OnFail
      (Development|PrintString "Did not find player")))
  (Utilities|FlowControl|Delay 1.0)
  (CallFunction|Moveto))

(event Custom|GoToPatrolPoints
  (AI|AIMoveTo self (Transformation|GetActorLocation (Utilities|Array|Get(acopy) (stale EventBeginPlay _outactors) (Variables|Default|GetCurrentPatrolPoint))) 0 5e+01 false ; Moves to player location
    (:OnSuccess
      (Development|PrintString "Found Player"))
    (:OnFail
      (Development|PrintString "Did not find player")))
  (bind _result (Math|Integer|IncrementInt (Variables|Default|GetCurrentPatrolPoint))
    (:%20%20
      (if (>= _result (Utilities|Array|Length (stale EventBeginPlay _outactors)))
        (Variables|Default|SetCurrentPatrolPoint 0)
        (Utilities|Array|Shuffle (stale EventBeginPlay _outactors))
        (else
          (Utilities|FlowControl|Delay 1.0)))
      (CallFunction|GotoPatrolPoints))))

(event EventBeginPlay
  (bind _outactors (Actor|GetAllActorsOfClasswithTag "/Script/Engine.Actor" "PatrolPoint"))
  (Development|PrintString (Utilities|String|Append "There are " (Utilities|String|ToString(Integer) (Utilities|Array|Length _outactors)) " patrol points"))
  (Utilities|Array|Shuffle _outactors)
  (Variables|/Script/Engine.CharacterMovementComponent|SetMaxWalkSpeed (Variables|Character|GetCharacterMovement) (Math|Conversions|ToFloat(Integer) (* (Math|Random|RandomIntegerinRange 8 12) 25)))
  (CallFunction|GotoPatrolPoints))

(fn ConstructionScript)